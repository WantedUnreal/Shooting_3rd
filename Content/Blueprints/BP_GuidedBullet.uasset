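; BP_GuidedBullet is a homing projectile that chases a random BP_Enemy.
; BeginPlay gathers all BP_Enemy actors and picks one at random as the target, with no retargeting afterward.
; Each Tick aims the local Z axis at the valid target, without turn smoothing, then moves along the up vector at Speed.
; Movement is unswept, and the graph has no hit handling.
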(event `self.ReceiveBeginPlay`
  (bind _outactors (`GameplayStatics.GetAllActorsOfClass` "/Game/Blueprints/BP_Enemy.BP_Enemy_C"))
  (bind _output_get (set `self.AllEnemy` _outactors))
  (bind _returnvalue (`KismetArrayLibrary.Array_Length` _output_get))
  (if (> _returnvalue 0)
    (set `self.TargetEnemy` (`|GetArrayItem` _output_get (`KismetMathLibrary.RandomIntegerInRange` 0 (- _returnvalue 1))))))

(event `self.ReceiveTick`
  (params (DeltaSeconds :type "Float (single-precision)"))
  (bind _targetenemy (`self.TargetEnemy`))
  (`|ExecutionSequence`
    (:`then_0`
      (`/Engine/EditorBlueprintResources/StandardMacros.IsValid` _targetenemy
        (:`Is Valid`
          (`self.K2_SetActorRotation` (`KismetMathLibrary.MakeRotFromZ` (- (`self.K2_GetActorLocation` _targetenemy) (`self.K2_GetActorLocation`)))))))
    (:`then_1`
      (`self.K2_SetActorLocation` (+ (`self.K2_GetActorLocation`) (* DeltaSeconds (* (`self.GetActorUpVector`) (`self.Speed`))))))))

(fn `UserConstructionScript`)