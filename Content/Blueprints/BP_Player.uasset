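; Player actor for a shooter that moves in the Y-Z plane via Enhanced Input and loads GameOver on any overlap.
; Tick drives movement and timed auto-fire from two muzzles, while IA_Fire spawns a guided bullet.
; Right mouse fires an instant radial ring of power bullets, spaced by an angle computed at BeginPlay.
; Key 1 spawns that ring sequentially, using a Delay inside Tick to pace each shot.
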(event `self.ReceiveBeginPlay`
  ; Enhanced Input 초기 설정
  (`EnhancedInputSubsystemInterface.AddMappingContext` (pcsubsystem `EnhancedInputLocalPlayerSubsystem` (`GameplayStatics.GetPlayerController` 0)) "/Game/Inputs/IMC_PlayerInput.IMC_PlayerInput" 0 (struct))
  ; Power Bullet 이 회전되야 하는 각도
  (set `self.PowerBulletAngle` (/ 360.0 (`self.PowerBulletCount`))))

(event `self.ReceiveTick`
  (params (DeltaSeconds :type "Float (single-precision)"))
  (`|ExecutionSequence`
    (:`then_0`
      (`self.Move` DeltaSeconds))
    (:`then_1`
      (`self.AutoFire` DeltaSeconds))
    (:`then_2`
      (if (`self.ActiveSkill1`)
        (`KismetSystemLibrary.Delay` 0.1)
        (`self.FireDelay360`)))))

(event `EnhancedInput|/Game/Inputs/IA_Fire`
  (params (ActionValue :type Boolean) (ElapsedSeconds :type "Float (double-precision)") (TriggeredSeconds :type "Float (double-precision)") (InputAction :type "InputAction Object Reference" :default "/Game/Inputs/IA_Fire.IA_Fire"))
  (:`Started`
    (`|SpawnActorFromClass` "/Game/Blueprints/BP_GuidedBullet.BP_GuidedBullet_C" (`self.GetTransform`) "Undefined" "MultiplyWithRoot" null null)))

(event `Key|RightMouseButton`
  (params (Key :type "Key Structure"))
  (:`Pressed`
    (`self.Fire360`)))

(event `Key|One`
  (params (Key :type "Key Structure"))
  (:`Pressed`
    (set `self.ActiveSkill1` true)))

(event `self.ReceiveActorBeginOverlap`
  (params (OtherActor :type "Actor Object Reference"))
  (`GameplayStatics.OpenLevel` "GameOver"))

(fn `AutoFire`
  (params (InputPin :type "Float (single-precision)"))
  ; 0.5 초 마다 총알을 발사하고 싶다.
  (bind _output_get (set `self.CurrTime` (+ (`self.CurrTime`) InputPin)))
  (if (> _output_get (`self.FireTime`))
    (`self.MakeBullet`)
    (set `self.CurrTime` 0.0)))

(fn `Fire360`
  (for _index (range (`self.PowerBulletCount`))
    (bind _returnvalue (`|SpawnActorFromClass` "/Game/Blueprints/BP_PowerBullet.BP_PowerBullet_C" (`SceneComponent.K2_GetComponentToWorld` (`self.FIrePos2`)) "Undefined" "MultiplyWithRoot" null null))
    (`self.K2_SetActorRotation` _returnvalue (`KismetMathLibrary.MakeRotator` (* _index (`self.PowerBulletAngle`))) false)))

(fn `FireDelay360`
  (bind _returnvalue (`|SpawnActorFromClass` "/Game/Blueprints/BP_PowerBullet.BP_PowerBullet_C" (`SceneComponent.K2_GetComponentToWorld` (`self.FIrePos2`)) "Undefined" "MultiplyWithRoot" null null))
  (`self.K2_SetActorRotation` _returnvalue (`KismetMathLibrary.MakeRotator` (* (`self.PowerBulletCurrCount`) (`self.PowerBulletAngle`))) false)
  (bind _output_get (set `self.PowerBulletCurrCount` (+ (`self.PowerBulletCurrCount`) 1)))
  (if (== _output_get (`self.PowerBulletCount`))
    (set `self.ActiveSkill1` false)
    (set `self.PowerBulletCurrCount` 0)))

(fn `MakeBullet`
  (`|SpawnActorFromClass` "/Game/Blueprints/BP_Bullet.BP_Bullet_C" (`SceneComponent.K2_GetComponentToWorld` (`self.FirePos`)) "Undefined" "MultiplyWithRoot" null null)
  (`|SpawnActorFromClass` "/Game/Blueprints/BP_Bullet.BP_Bullet_C" (`SceneComponent.K2_GetComponentToWorld` (`self.FirePos1`)) "Undefined" "MultiplyWithRoot" null null))

(fn `Move`
  (params (InputPin :type "Float (single-precision)"))
  (`self.K2_SetActorLocation` (+ (`self.K2_GetActorLocation`) (* InputPin (* (`KismetMathLibrary.Normal` (`KismetMathLibrary.MakeVector` 0.0 (`|GetInputActionValue`) (`|GetInputActionValue`))) (`self.Speed`))))))

(fn `UserConstructionScript`)