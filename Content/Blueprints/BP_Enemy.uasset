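; BP_Enemy is a shooting-game enemy that flies in a straight line and awards points when shot.
; On BeginPlay a random roll against TraceRate picks straight down or a one-time aim at BP_Player, rotating to face it; a missing player means down.
; Tick moves it along that direction at Speed.
; Overlapping an actor named like "Bullet" destroys both, spawns an explosion and adds Point to BP_ShootingGameState.
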(event `self.ReceiveBeginPlay`
  ; 1. 랜덤한 숫자를 뽑자 (0~9)
  ; 2. 만약에 0~2 (30%) 가 나왔으면
  ; 3. 방향을 아래로 설정
  ; 4. 그렇지 않으면(70%)
  ; 5. 방향을 플레이어를 향하는 방향으로 설정
  (if (< (`KismetMathLibrary.RandomIntegerInRange` 0 9) (`self.TraceRate`))
    (set `self.Direction` (0.0 0.0 -1.0) :!label _label)
    (else
      ;; 플레이어를 찾자.
      (bind _returnvalue (`GameplayStatics.GetActorOfClass` "/Game/Blueprints/BP_Player.BP_Player_C"))
      (bind _output_get (set `self.Target` _returnvalue))
      (`/Engine/EditorBlueprintResources/StandardMacros.IsValid` _output_get
        (:`Is Valid`
          ;; 플레이어를 향하는 방향 =
          ;; 플레이어 위치 - 나의 위치
          (bind _output_get_2 (set `self.Direction` (`KismetMathLibrary.Normal` (- (`self.K2_GetActorLocation` (`self.Target`)) (`self.K2_GetActorLocation`)))))
          (`self.K2_SetActorRotation` (`KismetMathLibrary.MakeRotFromZX` (* _output_get_2 -1.0) (`self.GetActorForwardVector`))))
        (:`Is Not Valid`
          (goto _label))))))

(event `self.ReceiveTick`
  (params (DeltaSeconds :type "Float (single-precision)"))
  (`self.K2_SetActorLocation` (+ (`self.K2_GetActorLocation`) (* DeltaSeconds (* (`self.Direction`) (`self.Speed`))))))

(event `self.ReceiveActorBeginOverlap`
  (params (OtherActor :type "Actor Object Reference"))
  ; 0. 만약에 부딪힌 물체가 Bullet 이라면
  ; 1. 나와 부딪힌 물체를 파괴하자.
  ; 2. 나의 위치에 파괴효과를 보여주자.
  ; 3. 나를 파괴하자.
  (if (`KismetStringLibrary.Contains` (`KismetSystemLibrary.GetDisplayName` OtherActor) "Bullet")
    (`self.K2_DestroyActor` OtherActor)
    (`GameplayStatics.SpawnEmitterAtLocation` "/Game/Realistic_Starter_VFX_Pack_Vol2/Particles/Destruction/P_Destruction_Electric.P_Destruction_Electric" (`self.K2_GetActorLocation`))
    (bind _asbp_shooting_game_state (cast `/Game/Blueprints/BP_ShootingGameState` (`GameplayStatics.GetGameState`)))
    (`/Game/Blueprints/BP_ShootingGameState.AddScore` _asbp_shooting_game_state (`self.Point`))
    (`self.K2_DestroyActor`)))

(fn `UserConstructionScript`)